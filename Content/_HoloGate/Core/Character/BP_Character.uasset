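; Player character Blueprint that handles movement and weapon firing through Enhanced Input.
; BeginPlay sets the weapon socket to absolute rotation, adds the input mapping context, binds an attribute-change delegate and initializes Health.
; Move input feeds CharacterMovement along world axes, while fire input starts and stops the weapon component.
; Cursor-based aiming with interpolated rotation for remote clients exists but is disconnected, and Tick does nothing.
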(event Custom|SetupBindings
  (bind _returnvalue (Class|HGCharacter|GetAttributesComponent))
  (EventDispatchers|BindEventtoOnAttributeChanged _returnvalue (EventDispatchers|CreateEvent (.AsBP%20HGPlayer%20Controller (Utilities|Casting|CastToBP_HGPlayerController (Class|HGCharacter|GetHGPlayerController))) :!event AttributeChanged))
  (Class|HGAttributesComponent|SetAttributeValue _returnvalue (GameplayTags|MakeLiteralGameplayTag "(TagName=\"Attribute.Health\")") 25.0))

(event Input|EnhancedActionEvents|EnhancedInputActionIA_Move
  (params (ActionValue :type Vector%202D%20Structure) (ElapsedSeconds :type Float%20%28double-precision%29) (TriggeredSeconds :type Float%20%28double-precision%29) (InputAction :type Input%20Action%20Object%20Reference :default "/Game/_HoloGate/Input/Actions/IA_Move.IA_Move"))
  (bind (_x _y) (Math|Vector2D|BreakVector2D ActionValue))
  (:Triggered
    (Class|PawnMovementComponent|AddInputVector (Variables|Character|GetCharacterMovement) (Math|Vector|MakeVector _x _y 0.0) false)))

(event Input|EnhancedActionEvents|EnhancedInputActionIA_Fire
  (params (ActionValue :type Boolean) (ElapsedSeconds :type Float%20%28double-precision%29) (TriggeredSeconds :type Float%20%28double-precision%29) (InputAction :type Input%20Action%20Object%20Reference :default "/Game/_HoloGate/Input/Actions/IA_Fire.IA_Fire"))
  (bind _returnvalue (Class|HGCharacter|GetWeaponComponent))
  (:Triggered
    (if ActionValue
      (Class|HGWeaponComponent|StartFiring _returnvalue)
      (else
        (Class|HGWeaponComponent|StopFiring _returnvalue)))))

(event EventBeginPlay
  (Variables|/Script/Engine.SceneComponent|SetbAbsoluteRotation (Class|HGCharacter|GetWeaponSocketComponent) true)
  (CallFunction|SetupBindings)
  (Input|AddMappingContext (PlayerController|LocalPlayerSubsystems|GetEnhancedInputLocalPlayerSubsystem (Class|HGCharacter|GetHGPlayerController)) "/Game/_HoloGate/Input/IMC_Character.IMC_Character" 0 "(bIgnoreAllPressedKeysUntilRelease=True,bForceImmediately=False)"))

(event EventTick
  (params (DeltaSeconds :type Float%20%28single-precision%29)))

(fn ConstructionScript)