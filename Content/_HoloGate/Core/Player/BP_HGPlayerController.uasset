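; BP_HGPlayerController is the player controller that owns the HUD and relays health changes to it.
; On BeginPlay it shows the mouse cursor, then creates W_HUD and adds it to the viewport.
; AttributeChanged switches on the gameplay tag and, for Health, sends the HUD the attribute entry looked up from the controlled BP_Character's attributes component, ignoring the event's old and new values.
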(event Custom|AttributeChanged
  (params (Attribute :type Gameplay%20Tag%20Structure) (OldValue :type Float%20%28single-precision%29) (NewValue :type Float%20%28single-precision%29))
  (bind _returnvalue (Pawn|GetControlledPawn))
  (bind _asbp_character (Utilities|Casting|CastToBP_Character _returnvalue))
  (bind _returnvalue_2 (Class|HGCharacter|GetAttributesComponent _asbp_character))
  ;[1 1 1] @TODO UI Component
  (|SwitchGameplayTag Attribute
    (:Attribute.Health
      (bind _w_hud (Variables|Default|GetW_HUD)
        (:then
          (Default|HealthChanged _w_hud (Utilities|Array|Get(acopy) (Variables|/Script/Case_HoloGate.HGAttributesComponent|GetAttributes _returnvalue_2) (Class|HGAttributesComponent|GetAttributeIndex _returnvalue_2 Attribute))))
        (:else)))))

(event EventBeginPlay
  ;[1 1 1] @TODO UI Component
  (Variables|Default|SetbShowMouseCursor true)
  (bind _returnvalue (UserInterface|CreateWidget "/Game/_HoloGate/UI/Widgets/W_HUD.W_HUD_C" self))
  (bind _output_get (Variables|Default|SetW_HUD _returnvalue))
  (UserInterface|Viewport|AddtoViewport _output_get 0))

(event EventTick
  (params (DeltaSeconds :type Float%20%28single-precision%29))
  ;[1 1 1] @TODO UI Component
)

(fn ConstructionScript)